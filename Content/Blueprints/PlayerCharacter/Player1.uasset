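; Player 1 character for a two-player bomb-placing game, which also receives and relays Player 2's input.
; P1 axis and bomb inputs call its own HorizontalMovement, VerticalMovement and SpawnBomb functions.
; P2 inputs look up the first Player2 actor on every event and call the same-named functions on it.
; P2 axes are crossed: horizontal input drives VerticalMovement and vertical input drives HorizontalMovement.
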(event EventBeginPlay
  (|CallParentFunction)
  (Development|PrintString "Player 1 ready"))

(event Collision|EventActorBeginOverlap
  (params (OtherActor :type Actor%20Object%20Reference)))

(event EventTick
  (params (DeltaSeconds :type Float%20%28single-precision%29)))

(event Input|ActionEvents|InputActionP1_PlaceBomb
  (params (Key :type Key%20Structure :default "AnyKey"))
  (:Pressed
    (CallFunction|SpawnBomb)))

(event Input|ActionEvents|InputActionP2_PlaceBomb
  (params (Key :type Key%20Structure :default "AnyKey"))
  (:Pressed
    (bind _outactors (Actor|GetAllActorsOfClass "/Game/Blueprints/PlayerCharacter/Player2.Player2_C"))
    (bind _asplayer_2 (Utilities|Casting|CastToPlayer2 (Utilities|Array|Get(acopy) _outactors)))
    (Default|SpawnBomb _asplayer_2)))

(event Input|AxisEvents|InputAxisP2_HorizontalMovement
  (params (AxisValue :type Float%20%28single-precision%29))
  (bind _outactors (Actor|GetAllActorsOfClass "/Game/Blueprints/PlayerCharacter/Player2.Player2_C"))
  (bind _asplayer_2 (Utilities|Casting|CastToPlayer2 (Utilities|Array|Get(acopy) _outactors)))
  (Default|VerticalMovement _asplayer_2 AxisValue (Input|AxisValues|GetP2_VerticalMovement)))

(event Input|AxisEvents|InputAxisP2_VerticalMovement
  (params (AxisValue :type Float%20%28single-precision%29))
  (bind _outactors (Actor|GetAllActorsOfClass "/Game/Blueprints/PlayerCharacter/Player2.Player2_C"))
  (bind _asplayer_2 (Utilities|Casting|CastToPlayer2 (Utilities|Array|Get(acopy) _outactors)))
  (Default|HorizontalMovement _asplayer_2 AxisValue (Input|AxisValues|GetP2_HorizontalMovement)))

(event Input|AxisEvents|InputAxisP1_HorizontalMovement
  (params (AxisValue :type Float%20%28single-precision%29))
  (CallFunction|HorizontalMovement AxisValue (Input|AxisValues|GetP1_VerticalMovement)))

(event Input|AxisEvents|InputAxisP1_VerticalMovement
  (params (AxisValue :type Float%20%28single-precision%29))
  (CallFunction|VerticalMovement AxisValue (Input|AxisValues|GetP1_HorizontalMovement)))

(fn ConstructionScript
  (|CallParentFunction))