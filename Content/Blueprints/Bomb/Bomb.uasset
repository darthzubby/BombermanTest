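; Bomberman-style bomb actor that flickers through a Delay chain on Tick, explodes in a cross, then resets the owning player's BombCount and destroys itself.
; BombExplosion multi-traces four directions up to BombStrength tiles, damaging hit actors until a Breakable or Unbreakable one ends that arm.
; The resulting tile distances drive ExplosionVisual, which stretches and reveals four blast meshes.
; BombCollider enables query and physics collision when an overlap ends.
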(event EventBeginPlay
  (Variables|ExplosionValues|SetBackwardValue 0)
  (Variables|ExplosionValues|SetForwardValue 0)
  (Variables|ExplosionValues|SetLeftValue 0)
  (Variables|ExplosionValues|SetRightValue 0)
  (Variables|ExplosionValues|SetForwardComplete false)
  (Variables|ExplosionValues|SetBackwardComplete false)
  (Variables|ExplosionValues|SetLeftComplete false)
  (Variables|ExplosionValues|SetRightComplete false))

(event EventTick
  (params (DeltaSeconds :type Float%20%28single-precision%29))
  (Utilities|FlowControl|Delay 1.0)
  (CallFunction|BombFlickeron)
  (Utilities|FlowControl|Delay 0.5)
  (CallFunction|BombFlickerOff)
  (Utilities|FlowControl|Delay 0.5)
  (CallFunction|BombFlickeron)
  (Utilities|FlowControl|Delay 0.5)
  (CallFunction|BombExplosion)
  (CallFunction|ExplosionVisual)
  (Utilities|FlowControl|Delay 0.5)
  (bind _asplayer_character (Utilities|Casting|CastToPlayerCharacter (Components|GetOwner)))
  (Variables|/Game/Blueprints/PlayerCharacter/PlayerCharacter.PlayerCharacter_C|SetBombCount _asplayer_character 1)
  (Actor|DestroyActor))

(event Collision|EventActorEndOverlap
  (params (OtherActor :type Actor%20Object%20Reference))
  (Collision|SetCollisionEnabled (Variables|Default|GetBombCollider) "QueryAndPhysics"))

(fn ConstructionScript)

(fn BombExplosion
  (bind _returnvalue (Transformation|GetActorLocation))
  (bind _returnvalue_2 (Transformation|GetActorLocation))
  (bind _returnvalue_3 (Transformation|GetActorLocation))
  (bind _returnvalue_4 (Transformation|GetActorLocation))
  (bind _bombstrength (Variables|BombStats|GetBombStrength))
  (bind _bombstrength_2 (Variables|BombStats|GetBombStrength))
  (bind _bombstrength_3 (Variables|BombStats|GetBombStrength))
  (bind _bombsphere (Variables|Default|GetBombSphere))
  (bind _bombstrength_4 (Variables|BombStats|GetBombStrength))
  (bind _bombsphere_2 (Variables|Default|GetBombSphere))
  (bind _bombsphere_3 (Variables|Default|GetBombSphere))
  (bind _bombsphere_4 (Variables|Default|GetBombSphere))
  (bind _returnvalue_5 (Transformation|GetWorldRotation _bombsphere))
  (bind _returnvalue_6 (Transformation|GetWorldRotation _bombsphere_2))
  (bind _returnvalue_7 (Transformation|GetWorldRotation _bombsphere_3))
  (bind _returnvalue_8 (Transformation|GetWorldRotation _bombsphere_4))
  (bind _returnvalue_9 (* _bombstrength_4 -100))
  (bind _returnvalue_10 (* _bombstrength_2 -100))
  (bind _returnvalue_11 (* _bombstrength_3 100))
  (bind _returnvalue_12 (* _bombstrength 100))
  (bind _returnvalue_13 (Math|Conversions|ToFloat(Integer) _returnvalue_11))
  (bind _returnvalue_14 (Math|Conversions|ToFloat(Integer) _returnvalue_9))
  (bind _returnvalue_15 (Math|Vector|GetForwardVector _returnvalue_7))
  (bind _returnvalue_16 (Math|Vector|GetForwardVector _returnvalue_6))
  (bind _returnvalue_17 (Math|Vector|GetRightVector _returnvalue_5))
  (bind _returnvalue_18 (Math|Vector|GetRightVector _returnvalue_8))
  (bind _returnvalue_19 (* _returnvalue_17 _returnvalue_14))
  (bind _returnvalue_20 (* _returnvalue_15 _returnvalue_10))
  (bind _returnvalue_21 (* _returnvalue_16 _returnvalue_12))
  (bind _returnvalue_22 (* _returnvalue_18 _returnvalue_13))
  (bind _returnvalue_23 (+ _returnvalue_4 _returnvalue_22))
  (bind _returnvalue_24 (+ _returnvalue_2 _returnvalue_19))
  (bind _returnvalue_25 (+ _returnvalue_21 _returnvalue_3))
  (bind _returnvalue_26 (+ _returnvalue _returnvalue_20))
  ;[1 1 1] RaycastForward
  (bind (_outhits _returnvalue_27) (Class|KismetSystemLibrary|LineTraceMultiforObjects _returnvalue_3 (Math|Vector|MakeVector (+ (.x _returnvalue_25) 5e+01) (.y _returnvalue_25) (.z _returnvalue_25)) (Utilities|Array|MakeArray "ObjectTypeQuery3" "ObjectTypeQuery2") false 0 "None" true))
  (if _returnvalue_27
    ;[1 1 1] Send Damage to Objects hit & Update the Explosion values
    (for _array_element _outhits
      (if (Math|Boolean|Equal(Boolean) (Variables|ExplosionValues|GetForwardComplete) false)
        (Class|TakeDamage|TakeDamage(Message) (.HitActor (Collision|BreakHitResult _array_element)) (Variables|BombStats|GetBombDamage))
        (if (or (Actor|ActorHasTag (.HitActor (Collision|BreakHitResult _array_element)) "Unbreakable") (Actor|ActorHasTag (.HitActor (Collision|BreakHitResult _array_element)) "Breakable"))
          (bind _newexplosionvalue (CallFunction|UpdateExplosionVisualValues (.HitActor (Collision|BreakHitResult _array_element)) self "Forward"))
          (Variables|ExplosionValues|SetForwardValue _newexplosionvalue)))))
  (if (Math|Boolean|Equal(Boolean) (Variables|ExplosionValues|GetForwardComplete) true)
    _
    (else
      (Variables|ExplosionValues|SetForwardValue (Variables|BombStats|GetBombStrength))))
  ;[1 1 1] RaycastBackward
  (bind (_outhits_2 _returnvalue_28) (Class|KismetSystemLibrary|LineTraceMultiforObjects _returnvalue (Math|Vector|MakeVector (+ (.x _returnvalue_26) -5e+01) (.y _returnvalue_26) (.z _returnvalue_26)) (Utilities|Array|MakeArray "ObjectTypeQuery3" "ObjectTypeQuery2") false 0 "None" true))
  (if _returnvalue_28
    ;[1 1 1] Send Damage to Objects hit
    (for _array_element_2 _outhits_2
      (if (Math|Boolean|Equal(Boolean) (Variables|ExplosionValues|GetBackwardComplete) false)
        (Class|TakeDamage|TakeDamage(Message) (.HitActor (Collision|BreakHitResult _array_element_2)) (Variables|BombStats|GetBombDamage))
        (if (or (Actor|ActorHasTag (.HitActor (Collision|BreakHitResult _array_element_2)) "Unbreakable") (Actor|ActorHasTag (.HitActor (Collision|BreakHitResult _array_element_2)) "Breakable"))
          (bind _newexplosionvalue_2 (CallFunction|UpdateExplosionVisualValues (.HitActor (Collision|BreakHitResult _array_element_2)) self "Backward"))
          (Variables|ExplosionValues|SetBackwardValue _newexplosionvalue_2)))))
  (if (Math|Boolean|Equal(Boolean) (Variables|ExplosionValues|GetBackwardComplete) true)
    _
    (else
      (Variables|ExplosionValues|SetBackwardValue (Variables|BombStats|GetBombStrength))))
  ;[1 1 1] RaycastRight
  (bind (_outhits_3 _returnvalue_29) (Class|KismetSystemLibrary|LineTraceMultiforObjects _returnvalue_4 (Math|Vector|MakeVector (.x _returnvalue_23) (+ (.y _returnvalue_23) 5e+01) (.z _returnvalue_23)) (Utilities|Array|MakeArray "ObjectTypeQuery3" "ObjectTypeQuery2") false 0 "None" true))
  (if _returnvalue_29
    ;[1 1 1] Send Damage to Objects hit
    (for _array_element_3 _outhits_3
      (if (Math|Boolean|Equal(Boolean) (Variables|ExplosionValues|GetRightComplete) false)
        (Class|TakeDamage|TakeDamage(Message) (.HitActor (Collision|BreakHitResult _array_element_3)) (Variables|BombStats|GetBombDamage))
        (if (or (Actor|ActorHasTag (.HitActor (Collision|BreakHitResult _array_element_3)) "Unbreakable") (Actor|ActorHasTag (.HitActor (Collision|BreakHitResult _array_element_3)) "Breakable"))
          (bind _newexplosionvalue_3 (CallFunction|UpdateExplosionVisualValues (.HitActor (Collision|BreakHitResult _array_element_3)) self "Right"))
          (Variables|ExplosionValues|SetRightValue _newexplosionvalue_3)))))
  (if (Math|Boolean|Equal(Boolean) (Variables|ExplosionValues|GetRightComplete) true)
    _
    (else
      (Variables|ExplosionValues|SetRightValue (Variables|BombStats|GetBombStrength))))
  ;[1 1 1] RaycastLeft
  (bind (_outhits_4 _returnvalue_30) (Class|KismetSystemLibrary|LineTraceMultiforObjects _returnvalue_2 (Math|Vector|MakeVector (.x _returnvalue_24) (+ (.y _returnvalue_24) -5e+01) (.z _returnvalue_24)) (Utilities|Array|MakeArray "ObjectTypeQuery3" "ObjectTypeQuery2") false 0 "None" true))
  (if _returnvalue_30
    ;[1 1 1] Send Damage to Objects hit
    (for _array_element_4 _outhits_4
      (if (Math|Boolean|Equal(Boolean) (Variables|ExplosionValues|GetLeftComplete) false)
        (Class|TakeDamage|TakeDamage(Message) (.HitActor (Collision|BreakHitResult _array_element_4)) (Variables|BombStats|GetBombDamage))
        (if (or (Actor|ActorHasTag (.HitActor (Collision|BreakHitResult _array_element_4)) "Unbreakable") (Actor|ActorHasTag (.HitActor (Collision|BreakHitResult _array_element_4)) "Breakable"))
          (bind _newexplosionvalue_4 (CallFunction|UpdateExplosionVisualValues (.HitActor (Collision|BreakHitResult _array_element_4)) self "Left"))
          (Variables|ExplosionValues|SetLeftValue _newexplosionvalue_4)))))
  (if (not (Math|Boolean|Equal(Boolean) (Variables|ExplosionValues|GetLeftComplete) true))
    (Variables|ExplosionValues|SetLeftValue (Variables|BombStats|GetBombStrength))))

(fn UpdateExplosionVisualValues
  (params (CurrentActor :type Actor%20Object%20Reference) (PreviousActor :type Actor%20Object%20Reference) (ExplosionDirection :type String))
  (switch string ExplosionDirection
    (:Default
      _)
    (:Forward
      (Variables|ExplosionValues|SetForwardComplete true))
    (:Backward
      (Variables|ExplosionValues|SetBackwardComplete true))
    (:Right
      (Variables|ExplosionValues|SetRightComplete true))
    (:Left
      (Variables|ExplosionValues|SetLeftComplete true)))
  (return (Math|Float|Round (/ (Math|Vector|VectorLength (- (Transformation|GetActorLocation PreviousActor) (Transformation|GetActorLocation CurrentActor))) 1e+02))))

(fn ExplosionVisual
  ;[1 1 1] Update objects position and scale based on explosion values
  (Transformation|SetRelativeTransform (Variables|Default|GetForwardExplosion) (Math|Transform|MakeTransform (Math|Vector|MakeVector (/ (- (* (+ (Variables|ExplosionValues|GetForwardValue) 1) 1e+02) 5e+01) 2.0) 0.0 0.0) "0,90.000000,90.000000" (Math|Vector|MakeVector 0.5 0.5 (- (Math|Conversions|ToFloat(Integer) (+ (Variables|ExplosionValues|GetForwardValue) 1)) 0.5))) false false)
  (Transformation|SetRelativeTransform (Variables|Default|GetBackwardExplosion) (Math|Transform|MakeTransform (Math|Vector|MakeVector (/ (- (* (+ (Variables|ExplosionValues|GetBackwardValue) 1) -1e+02) -5e+01) 2.0) 0.0 0.0) "0.000000,90.000000,90.000000" (Math|Vector|MakeVector 0.5 0.5 (- (Math|Conversions|ToFloat(Integer) (+ (Variables|ExplosionValues|GetBackwardValue) 1)) 0.5))) false false)
  (Transformation|SetRelativeTransform (Variables|Default|GetLeftExplosion) (Math|Transform|MakeTransform (Math|Vector|MakeVector 0.0 (/ (- (* (+ (Variables|ExplosionValues|GetLeftValue) 1) -1e+02) -5e+01) 2.0) 0.0) "0, 0,90.000000" (Math|Vector|MakeVector 0.5 0.5 (- (Math|Conversions|ToFloat(Integer) (+ (Variables|ExplosionValues|GetLeftValue) 1)) 0.5))) false false)
  (Transformation|SetRelativeTransform (Variables|Default|GetRightExplosion) (Math|Transform|MakeTransform (Math|Vector|MakeVector 0.0 (/ (- (* (+ (Variables|ExplosionValues|GetRightValue) 1) 1e+02) 5e+01) 2.0) 0.0) "0, 0,90.000000" (Math|Vector|MakeVector 0.5 0.5 (- (Math|Conversions|ToFloat(Integer) (+ (Variables|ExplosionValues|GetRightValue) 1)) 0.5))) false false)
  ;[1 1 1] Set Explosion Visibility
  (Rendering|SetVisibility (Variables|Default|GetForwardExplosion) true false)
  (Rendering|SetVisibility (Variables|Default|GetBackwardExplosion) true false)
  (Rendering|SetVisibility (Variables|Default|GetLeftExplosion) true false)
  (Rendering|SetVisibility (Variables|Default|GetRightExplosion) true false))

(fn BombFlickeron
  (Rendering|Material|SetMaterial (Variables|Default|GetBombSphere) 0 "/Game/Material/BombReady.BombReady")
  (Rendering|Material|SetMaterial (Variables|Default|GetBombTop) 0 "/Game/Material/BombReady.BombReady"))

(fn BombFlickerOff
  (Rendering|Material|SetMaterial (Variables|Default|GetBombSphere) 0 "/Game/Material/BombMain.BombMain")
  (Rendering|Material|SetMaterial (Variables|Default|GetBombTop) 0 "/Game/Material/BombMain.BombMain"))